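; Player character with Enhanced Input movement, look, sprint, crouch and a camera-mounted shotgun.
; BeginPlay adds the input mapping context, then spawns BP_Shotgun and snaps it to the camera.
; Firing calls the shotgun's fire function and spawns a BP_ShotgunShell at its muzzle point.
; Run press and release both flip walk speed for hold-to-sprint, crouch toggles per press, and look input scales by delta time and per-axis sensitivity.
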(event `self.ReceiveBeginPlay`
  (`|ExecutionSequence`
    (:`then_0`
      (`EnhancedInputSubsystemInterface.AddMappingContext` (pcsubsystem `EnhancedInputLocalPlayerSubsystem` (`GameplayStatics.GetPlayerController` 0)) "/Game/Core/Input/IMC_Main.IMC_Main" 0 (struct)))
    (:`then_1`
      ;[1 0.5885 0.978 0.5] Spawn Shotgun
      (bind _returnvalue (`|SpawnActorFromClass` "/Game/Weapons/Scripts/BP_Shotgun.BP_Shotgun_C" (`KismetMathLibrary.MakeTransform` (0.0 0.0 0.0)) "Undefined" "MultiplyWithRoot" null null))
      (bind _output_get (set `self.ShotgunRef` _returnvalue))
      (`self.K2_AttachToComponent` _output_get (`self.Camera`) "None" "SnapToTarget" "SnapToTarget" "SnapToTarget" true))))

(event `EnhancedInput|/Game/Core/Input/IA_Fire`
  (params (ActionValue :type Boolean) (ElapsedSeconds :type "Float (double-precision)") (TriggeredSeconds :type "Float (double-precision)") (InputAction :type "InputAction Object Reference" :default "/Game/Core/Input/IA_Fire.IA_Fire"))
  (bind (_returnvalue_location _returnvalue_rotation) (`KismetMathLibrary.BreakTransform` (`SceneComponent.K2_GetComponentToWorld` (`/Game/Weapons/Scripts/BP_Shotgun.MuzzlePoint` (`self.ShotgunRef`)))))
  ;[1 0.5885 0.978 0.5] Fire
  (:`Triggered`
    (`/Game/Weapons/Scripts/BP_Shotgun.Fireshotgun` (`self.ShotgunRef`))
    (`|SpawnActorFromClass` "/Game/Weapons/1887_shotgun/BP_ShotgunShell.BP_ShotgunShell_C" (`KismetMathLibrary.MakeTransform` _returnvalue_location _returnvalue_rotation) "Undefined" "MultiplyWithRoot" null null)))

(event `EnhancedInput|/Game/Core/Input/IA_Move`
  (params (ActionValue :type "Vector2D Structure") (ElapsedSeconds :type "Float (double-precision)") (TriggeredSeconds :type "Float (double-precision)") (InputAction :type "InputAction Object Reference" :default "/Game/Core/Input/IA_Move.IA_Move"))
  (bind (_x _y) (`KismetMathLibrary.BreakVector2D` ActionValue))
  (:`Triggered`
    (`self.AddMovementInput` (`self.GetActorForwardVector`) _y)
    (`self.AddMovementInput` (`self.GetActorRightVector`) _x)))

(event `EnhancedInput|/Game/Core/Input/IA_Look`
  (params (ActionValue :type "Vector2D Structure") (ElapsedSeconds :type "Float (double-precision)") (TriggeredSeconds :type "Float (double-precision)") (InputAction :type "InputAction Object Reference" :default "/Game/Core/Input/IA_Look.IA_Look"))
  (bind (_x _y) (`KismetMathLibrary.BreakVector2D` ActionValue))
  (:`Triggered`
    (`self.AddControllerYawInput` (* (* _x (`GameplayStatics.GetWorldDeltaSeconds`)) (`self.Sensitivity X`)))
    (`self.AddControllerPitchInput` (* (* _y (`GameplayStatics.GetWorldDeltaSeconds`)) (`self.Sensitivity Y`)))))

(event `EnhancedInput|/Game/Core/Input/IA_Run`
  (params (ActionValue :type Boolean) (ElapsedSeconds :type "Float (double-precision)") (TriggeredSeconds :type "Float (double-precision)") (InputAction :type "InputAction Object Reference" :default "/Game/Core/Input/IA_Run.IA_Run"))
  (bind _charactermovement (`self.CharacterMovement`))
  (:`Started`
    (if (`self.isRunning`) :!label _label
      (set `CharacterMovementComponent.MaxWalkSpeed` 600.0 _charactermovement)
      (set `self.isRunning` false)
      (`KismetSystemLibrary.PrintString` "walking")
      (else
        (set `CharacterMovementComponent.MaxWalkSpeed` 1000.0 _charactermovement)
        (set `self.isRunning` true)
        (`KismetSystemLibrary.PrintString` "sprinting"))))
  (:`Completed`
    (goto _label)))

(event `EnhancedInput|/Game/Core/Input/IA_Crouch`
  (params (ActionValue :type Boolean) (ElapsedSeconds :type "Float (double-precision)") (TriggeredSeconds :type "Float (double-precision)") (InputAction :type "InputAction Object Reference" :default "/Game/Core/Input/IA_Crouch.IA_Crouch"))
  (:`Started`
    (if (`NavMovementComponent.IsCrouching` (`self.CharacterMovement`))
      (`self.UnCrouch`)
      (`KismetSystemLibrary.PrintString` "stand")
      (else
        (`self.Crouch`)
        (`KismetSystemLibrary.PrintString` "crouch")))))

(fn `UserConstructionScript`)