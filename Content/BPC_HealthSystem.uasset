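; BPC_HealthSystem is a health component that tracks current health against a maximum, starting full on BeginPlay.
; HealthIncrease fires the EDUpdatedHealth dispatcher before adding healing clamped between zero and MaxHealth, so listeners are notified before the value changes.
; DecreaseHealth subtracts damage without clamping, then fires the same dispatcher.
; Death at zero or below is only a "die" debug print.
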(event `self.ReceiveBeginPlay`
  (set `self.Current health` (`self.Max Health`)))

(fn `DecreaseHealth`
  (params (Damage :type Integer))
  (bind _output_get (set `self.Current health` (- (`self.Current health`) Damage)))
  (`self.ED_UpdatedHealth`)
  (if (<= _output_get 0)
    (`KismetSystemLibrary.PrintString` "die")))

(fn `HealthIncrease`
  (params (Healing :type Integer))
  (`self.ED_UpdatedHealth`)
  (set `self.Current health` (`KismetMathLibrary.Clamp` (+ (`self.Current health`) Healing) 0 (`self.Max Health`))))